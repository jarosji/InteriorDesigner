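; Test actor that exercises the JJ runtime asset and HTTP features through debug keys, enabling input on BeginPlay and hiding its Plane.
; T asynchronously imports a hardcoded PNG and applies it to the Plane through a dynamic material instance.
; C logs into a localhost server, then prints fetched file descriptions or the failure code.
; M imports a chosen OBJ/FBX and spawns a runtime mesh actor; procedural-mesh and export calls are unwired.
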(event `self.ReceiveBeginPlay`
  (`self.EnableInput` (`GameplayStatics.GetPlayerController` 0))
  (`SceneComponent.SetVisibility` (`self.Plane`) false true))

(event `Key|T`
  (params (Key :type "Key Structure"))
  (bind _plane (`self.Plane`))
  (:`Pressed`
    (bind _texture (`ImportTextureAsync.ImportTextureAsync` "C:\\Users\\JJ\\Desktop\\tex\\window.png")
      (:`OnTextureImported`
        (bind _returnvalue (`PrimitiveComponent.CreateDynamicMaterialInstance` _plane 0 (`PrimitiveComponent.GetMaterial` _plane 0) "None"))
        (`PrimitiveComponent.SetMaterial` _plane 0 _returnvalue)
        (`MaterialInstanceDynamic.SetVectorParameterValue` _returnvalue "DiffuseColor" (struct :`R` 1.0 :`G` 1.0 :`B` 1.0 :`A` 1.0))
        (`MaterialInstanceDynamic.SetTextureParameterValue` _returnvalue "TextureD" _texture)))))

(event `self.ReceiveTick`
  (params (DeltaSeconds :type "Float (single-precision)")))

(event `Key|C`
  (params (Key :type "Key Structure"))
  (bind _returnvalue (subsystem `JJHttpSubsystem`))
  (:`Pressed`
    (`JJHttpSubsystem.Logout` _returnvalue)
    (`JJHttpSubsystem.Login` _returnvalue "https://localhost:7004/User/Login" "Test1" "1234" (delegate `CustomEvent_0`) (delegate `CustomEvent_1`))))

(event `CustomEvent_1`
  (params (StatucCode :type Integer))
  (`KismetSystemLibrary.PrintString` (`KismetStringLibrary.Conv_IntToString` StatucCode)))

(event `CustomEvent_0`
  (params (UserInfo :type "UserInfo Structure") (BearerToken :type String))
  (bind _filedesc (`FetchFileDescriptions.FetchFileDescriptions`)
    (:`OnFileDescriptionsFetched`
      (for _array_element _filedesc
        (`KismetSystemLibrary.PrintString` (break `File` _array_element))))))

(event `Key|M`
  (params (Key :type "Key Structure"))
  (:`Pressed`
    (bind (_filepath _returnvalue) (`JJFileDialogLibrary.OpenFileDialog` "" "" (`|MakeArray` "obj | fbx") (`|MakeArray` "3D Model (.obj, .fbx)")))
    (if _returnvalue
      (bind (_modelwrapper _bissuccess) (`ImportModelAsync.ImportModelAsync` _filepath)
        (:`OnJJModelImported`
          (if _bissuccess
            (`SpawnRuntimeMeshActorAsync.SpawnRuntimeMeshActorAsync` _modelwrapper)))))))

(event `CustomEvent`
  (params (FileStateOut :type "SourceControlState Structure"))
  ;[1 1 1] Funkce s údálostí jako parametr
)

(fn `ConstructProceduralMesh`
  (params (ModelWrapper :type "JJModelWrapper Object Reference"))
  (locals (ProceduralMeshComponent :type "ProceduralMeshComponent Object Reference"))
  (bind _modelwrapper (`local.ModelWrapper`))
  (bind _returnvalue (`AddComponent|NODE_AddProceduralMeshComponent-1`))
  (set `local.ProceduralMeshComponent` _returnvalue)
  (for _index (range (`JJModelWrapper.GetNumberOfSections` (`local.ModelWrapper`)))
    (`ProceduralMeshComponent.CreateMeshSection_LinearColor` :`self` (`local.ProceduralMeshComponent`) :`SectionIndex` _index :`Vertices` (`JJModelWrapper.GetPositions` _modelwrapper _index) :`Triangles` (`JJModelWrapper.GetIndices` _modelwrapper _index) :`Normals` (`JJModelWrapper.GetNormals` _modelwrapper _index) :`bCreateCollision` true)))

(fn `UserConstructionScript`)