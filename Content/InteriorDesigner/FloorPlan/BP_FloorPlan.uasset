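; BP_FloorPlan displays a floor plan texture on a sizable plane for the interior designer.
; On BeginPlay it scales the Plane from Size, assuming a 100-unit base mesh, and applies a dynamic material instance with Texture as its "Texture" parameter.
; SetSize stores a new size and rescales the Plane at runtime.
; The construction script is empty, so size and texture take effect only during play.
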(event `self.ReceiveBeginPlay`
  (bind _plane (`self.Plane`))
  (bind (_returnvalue_x _returnvalue_y) (`KismetMathLibrary.BreakVector2D` (/ (`self.Size`) (100.0 100.0))))
  (`SceneComponent.SetWorldScale3D` _plane (`KismetMathLibrary.MakeVector` _returnvalue_x _returnvalue_y 1.0))
  (bind _returnvalue (`KismetMaterialLibrary.CreateDynamicMaterialInstance` (`PrimitiveComponent.GetMaterial` _plane 0)))
  (`PrimitiveComponent.SetMaterial` _plane 0 _returnvalue)
  (`MaterialInstanceDynamic.SetTextureParameterValue` _returnvalue "Texture" (`self.Texture`)))

(fn `SetSize`
  (params (NewSize :type "Vector2D Structure"))
  (bind _output_get (set `self.Size` NewSize))
  (bind (_returnvalue_x _returnvalue_y) (`KismetMathLibrary.BreakVector2D` (/ _output_get (100.0 100.0))))
  (`SceneComponent.SetWorldScale3D` (`self.Plane`) (`KismetMathLibrary.MakeVector` _returnvalue_x _returnvalue_y 1.0)))

(fn `UserConstructionScript`)