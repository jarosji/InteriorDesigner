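; Transform gizmo for the interior designer that lifts and rotates the selected actor, shown only while a selection exists.
; An arrow widget floats above the actor facing the pawn; dragging it moves the actor vertically via mouse-ray/plane intersection deltas.
; A circle-material plane scales to the actor's bounds, and left-dragging near its rim sets yaw from the look-at angle toward the cursor hit.
; Tick drives placement, cursor feedback and both manipulations.
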(event `self.ReceiveBeginPlay`
  (bind _returnvalue (`GameplayStatics.GetPlayerController` 0))
  (add `InteriorDesignerSubsystem.OnSelectionChanged` (subsystem `InteriorDesignerSubsystem`) (delegate `CustomEvent`))
  (bind _aswbp_single_arrow_gizmo (cast `/Game/InteriorDesigner/Gizmo/WBP_SingleArrowGizmo` (`WidgetComponent.GetWidget` (`self.Widget`))))
  (add `/Game/InteriorDesigner/Gizmo/WBP_SingleArrowGizmo.OnPressed` _aswbp_single_arrow_gizmo (delegate `OnPressed_Event`))
  (add `/Game/InteriorDesigner/Gizmo/WBP_SingleArrowGizmo.OnReleased` _aswbp_single_arrow_gizmo (delegate `OnReleased_Event`))
  (bind _returnvalue_2 (`PrimitiveComponent.CreateDynamicMaterialInstance` (`self.Plane`) 0 "/Game/InteriorDesigner/Gizmo/M_GizmoCircle.M_GizmoCircle" "None"))
  (set `self.NewVar` _returnvalue_2)
  (set `PlayerController.bEnableClickEvents` true _returnvalue)
  (set `PlayerController.bEnableMouseOverEvents` true _returnvalue))

(event `OnPressed_Event`
  (bind (_worldlocation _worlddirection) (`PlayerController.DeprojectMousePositionToWorld` (`GameplayStatics.GetPlayerController` 0)))
  (set `self.Translating` true)
  (set `self.Old` (`.Intersection` (`KismetMathLibrary.LinePlaneIntersection_OriginNormal` _worldlocation (+ _worldlocation (* _worlddirection 10000.0)) (`self.GetActorBounds` (`InteriorDesignerSubsystem.GetSelectedActor` (subsystem `InteriorDesignerSubsystem`)) false false) (`self.GetActorForwardVector` (`InteriorDesignerSubsystem.GetSelectedActor` (subsystem `InteriorDesignerSubsystem`)))))))

(event `OnReleased_Event`
  (set `self.Translating` false))

(event `CustomEvent`
  (params (SelectedActor :type "Actor Object Reference"))
  (`SceneComponent.SetVisibility` (`self.DefaultSceneRoot`) (`KismetSystemLibrary.IsValid` SelectedActor) true))

(event `self.ReceiveTick`
  (params (DeltaSeconds :type "Float (single-precision)"))
  (bind _returnvalue (`GameplayStatics.GetPlayerController` 0))
  (bind _plane (`self.Plane`))
  (bind _widget (`self.Widget`))
  (bind _returnvalue_2 (`InteriorDesignerSubsystem.GetSelectedActor` (subsystem `InteriorDesignerSubsystem`)))
  (bind _returnvalue_3 (`InteriorDesignerSubsystem.GetSelectedActor` (subsystem `InteriorDesignerSubsystem`)))
  (bind _returnvalue_4 (`InteriorDesignerSubsystem.GetSelectedActor` (subsystem `InteriorDesignerSubsystem`)))
  (bind _hitresult (`PlayerController.GetHitResultUnderCursorByChannel` (`GameplayStatics.GetPlayerController` 0) "TraceTypeQuery1" true))
  (bind (_worldlocation _worlddirection) (`PlayerController.DeprojectMousePositionToWorld` (`GameplayStatics.GetPlayerController` 0)))
  (bind (_returnvalue_roll _returnvalue_pitch) (`KismetMathLibrary.BreakRotator` (`self.K2_GetActorRotation` _returnvalue_2)))
  (bind (_origin _boxextent) (`self.GetActorBounds` _returnvalue_4 false false))
  (bind (_returnvalue_x _returnvalue_y _returnvalue_z) (`KismetMathLibrary.BreakVector` (`self.K2_GetActorLocation` (`InteriorDesignerSubsystem.GetSelectedActor` (subsystem `InteriorDesignerSubsystem`)))))
  (bind (_returnvalue_roll_2 _returnvalue_pitch_2 _returnvalue_yaw) (`KismetMathLibrary.BreakRotator` (`KismetMathLibrary.FindLookAtRotation` (`self.K2_GetActorLocation` _returnvalue_2) (`self.MousePos`))))
  (bind (_origin_2 _boxextent_2 _sphereradius) (`KismetSystemLibrary.GetComponentBounds` (`Actor.RootComponent` (`InteriorDesignerSubsystem.GetSelectedActor` (subsystem `InteriorDesignerSubsystem`)))))
  (bind (_returnvalue_roll_3 _returnvalue_pitch_3 _returnvalue_yaw_2) (`KismetMathLibrary.BreakRotator` (`KismetMathLibrary.FindLookAtRotation` (`self.K2_GetActorLocation` (`InteriorDesignerSubsystem.GetSelectedActor` (subsystem `InteriorDesignerSubsystem`))) (`self.MousePos`))))
  (bind (_t _intersection) (`KismetMathLibrary.LinePlaneIntersection_OriginNormal` _worldlocation (+ _worldlocation (* _worlddirection 10000.0)) _origin (`self.GetActorForwardVector` _returnvalue_3)))
  (bind _returnvalue_5 (/ (`.SphereRadius` (`KismetSystemLibrary.GetComponentBounds` (`Actor.RootComponent` (`InteriorDesignerSubsystem.GetSelectedActor` (subsystem `InteriorDesignerSubsystem`))))) 50.0))
  (bind (_returnvalue_x_2 _returnvalue_y_2 _returnvalue_z_2) (`KismetMathLibrary.BreakVector` (- _intersection (`self.Old`))))
  (`/Engine/EditorBlueprintResources/StandardMacros.IsValid` _returnvalue_4
    (:`Is Valid`
      (`|ExecutionSequence`
        (:`then_0`
          (bind _returnvalue_6 (`GameplayStatics.GetActorOfClass` "/Game/InteriorDesigner/Core/PlayerInput/IDFloatingPawn.IDFloatingPawn_C"))
          (`SceneComponent.K2_SetWorldLocationAndRotation` _widget (+ _origin (`KismetMathLibrary.MakeVector` 0.0 0.0 (+ (.z _boxextent) 15.0))) (`KismetMathLibrary.FindLookAtRotation` (`SceneComponent.K2_GetComponentLocation` _widget) (`self.K2_GetActorLocation` _returnvalue_6)) false false))
        (:`then_1`
          (if (`self.Translating`)
            (`self.K2_AddActorWorldOffset` _returnvalue_3 (`KismetMathLibrary.MakeVector` 0.0 0.0 _returnvalue_z_2) false false)
            (set `self.Old` _intersection)))
        (:`then_2`
          (`SceneComponent.K2_SetWorldLocation` _plane (`KismetMathLibrary.MakeVector` _returnvalue_x _returnvalue_y _returnvalue_z) false false)
          (`SceneComponent.SetWorldScale3D` _plane (`KismetMathLibrary.MakeVector` _returnvalue_5 _returnvalue_5 0.001)))
        (:`then_3`
          (set `self.MousePos` (`.Location` (`GameplayStatics.BreakHitResult` _hitresult)))
          (if (and (== (`.HitComponent` (`GameplayStatics.BreakHitResult` _hitresult)) (`self.Plane`)) (`KismetMathLibrary.InRange_FloatFloat` (`KismetMathLibrary.Distance2D` (`KismetMathLibrary.Conv_VectorToVector2D` (`.Location` (`GameplayStatics.BreakHitResult` _hitresult))) (`KismetMathLibrary.Conv_VectorToVector2D` _origin_2)) (- _sphereradius 4.0) (+ _sphereradius 4.0)))
            (set `PlayerController.CurrentMouseCursor` "GrabHand" _returnvalue)
            (bind _asidfloating_pawn (cast `/Game/InteriorDesigner/Core/PlayerInput/IDFloatingPawn` (`Controller.K2_GetPawn` (`GameplayStatics.GetPlayerController` 0))))
            (if (`/Game/InteriorDesigner/Core/PlayerInput/IDFloatingPawn.IsLeftButtonDown` _asidfloating_pawn)
              (set `self.Rotating` true)
              (set `self.OldRot` _returnvalue_yaw_2))
            (else
              (bind _asidfloating_pawn_2 (cast `/Game/InteriorDesigner/Core/PlayerInput/IDFloatingPawn` (`Controller.K2_GetPawn` (`GameplayStatics.GetPlayerController` 0))))
              (if (not (`/Game/InteriorDesigner/Core/PlayerInput/IDFloatingPawn.IsLeftButtonDown` _asidfloating_pawn_2))
                (set `PlayerController.CurrentMouseCursor` "Default" _returnvalue)
                (set `self.Rotating` false)))))
        (:`then_4`
          (if (`self.Rotating`)
            (`self.K2_SetActorRotation` _returnvalue_2 (`KismetMathLibrary.MakeRotator` _returnvalue_roll _returnvalue_pitch (- _returnvalue_yaw (`self.OldRot`))) false)))))))

(fn `UserConstructionScript`)